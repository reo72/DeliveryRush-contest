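; BP_EvaluationManager rates a delivery from 1 to 5 stars and opens WBP_ResultScreen.
; Delivery time sets the base rating, adjusted by cargo integrity, accumulated obstacle hits and a detour penalty.
; As wired, intact cargo adds a star without clamping or showing results, while damaged cargo does both only per hit or detour penalty.
; OnTimeLimitExceeded clears its flag before evaluating, so it bypasses the one-star timeout branch.
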(event EventBeginPlay)

(event EventTick
  (params (DeltaSeconds :type Float%20%28single-precision%29)))

(fn CalculateEvaluation
  (if (Variables|Default|GetTimeLimitExceeded)
    (Variables|Default|SetStarRating 1)
    (CallFunction|ShowResult)
    (else
      (if (<= (Variables|Default|GetDeliveryTime) 2e+01)
        (Variables|Default|SetStarRating 5)
        (elif (<= (Variables|Default|GetDeliveryTime) 3e+01)
          (Variables|Default|SetStarRating 4)
          (elif (<= (Variables|Default|GetDeliveryTime) 4e+01)
            (Variables|Default|SetStarRating 3)
            (elif (<= (Variables|Default|GetDeliveryTime) 5e+01)
              (Variables|Default|SetStarRating 2)
              (else
                (Variables|Default|SetStarRating 1))))))
      (if (>= (Variables|Default|GetCargoIntegrity) 1e+02)
        (Variables|Default|SetStarRating (+ (Variables|Default|GetStarRating) 1))
        (else
          (for _index (range 0 (- (Variables|Default|GetObstacleHitCount) 1))
            (Variables|Default|SetStarRating (- (Variables|Default|GetStarRating) 1))
            (Variables|Default|SetStarRating (Math|Integer|Clamp(Integer) (Variables|Default|GetStarRating) 1 5))
            (CallFunction|ShowResult))
          (if (Variables|Default|GetDetourPenaltyApplied)
            (Variables|Default|SetStarRating (- (Variables|Default|GetStarRating) 1))
            (Variables|Default|SetStarRating (Math|Integer|Clamp(Integer) (Variables|Default|GetStarRating) 1 5))
            (CallFunction|ShowResult)))))))

(fn ShowResult
  (bind _returnvalue (UserInterface|CreateWidget "/Game/UI/WBP_ResultScreen.WBP_ResultScreen_C"))
  (UserInterface|Viewport|AddtoViewport _returnvalue 0))

(fn OnDeliveryComplete
  (CallFunction|CalculateEvaluation))

(fn OnTimeLimitExceeded
  (Variables|Default|SetTimeLimitExceeded false)
  (CallFunction|CalculateEvaluation))

(fn ApplyObstacleHit
  (Variables|Default|SetObstacleHitCount (+ (Variables|Default|GetObstacleHitCount) 1)))

(fn ApplyCargoDamage
  (params (DamageAmount :type Float%20%28double-precision%29))
  (Variables|Default|SetCargoIntegrity (- (Variables|Default|GetCargoIntegrity) DamageAmount)))