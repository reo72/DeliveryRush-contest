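; BP_DeliveryPoint is a drop-off actor where the player completes delivery orders.
; Overlap enables input and shows the WB_DeliverPrompt widget; leaving disables input and removes it.
; Pressing F checks that TargetRowName matches CurrentTargetName in BP_DeliveryGameInstance and that PlayerInventory is not empty.
; Success increments CompletedOrders, generates a new order and removes the prompt, while failures only print a Japanese message.
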(event EventBeginPlay)

(event Collision|EventActorBeginOverlap
  (params (OtherActor :type Actor%20Object%20Reference))
  (Input|EnableInput (Game|GetPlayerController 0))
  (Variables|Default|SetbPlayerNearby true)
  (bind _returnvalue (UserInterface|CreateWidget "/Game/MJ/system/WB_DeliverPrompt.WB_DeliverPrompt_C"))
  (bind _output_get (Variables|Default|SetDeliveryWidget _returnvalue))
  (UserInterface|Viewport|AddtoViewport _output_get 0))

(event EventTick
  (params (DeltaSeconds :type Float%20%28single-precision%29)))

(event Collision|EventActorEndOverlap
  (params (OtherActor :type Actor%20Object%20Reference))
  (Input|DisableInput (Game|GetPlayerController 0))
  (Variables|Default|SetbPlayerNearby false)
  (Utilities|IsValid (Variables|Default|GetDeliveryWidget)
    (:Is%20Valid
      (Widget|RemovefromParent (Variables|Default|GetDeliveryWidget)))))

(event Input|KeyboardEvents|F
  (params (Key :type Key%20Structure :default "None"))
  (:Pressed
    (if (Variables|Default|GetbPlayerNearby)
      (bind _asbp_delivery_game_instance (Utilities|Casting|CastToBP_DeliveryGameInstance (Game|GetGameInstance)))
      (if (== (Variables|/Game/MJ/system/BP_DeliveryGameInstance.BP_DeliveryGameInstance_C|GetCurrentTargetName _asbp_delivery_game_instance) (Variables|Default|GetTargetRowName))
        (if (Utilities|Array|IsEmpty (Variables|/Game/MJ/system/BP_DeliveryGameInstance.BP_DeliveryGameInstance_C|GetPlayerInventory _asbp_delivery_game_instance))
          (Development|PrintString "商品を持っていません")
          (else
            (Development|PrintString "配達完了！")
            (Variables|/Game/MJ/system/BP_DeliveryGameInstance.BP_DeliveryGameInstance_C|SetbHasActiveOrder _asbp_delivery_game_instance (Variables|/Game/MJ/system/BP_DeliveryGameInstance.BP_DeliveryGameInstance_C|GetbHasActiveOrder _asbp_delivery_game_instance))
            (Variables|/Game/MJ/system/BP_DeliveryGameInstance.BP_DeliveryGameInstance_C|SetCompletedOrders _asbp_delivery_game_instance (+ (Variables|/Game/MJ/system/BP_DeliveryGameInstance.BP_DeliveryGameInstance_C|GetCompletedOrders _asbp_delivery_game_instance) 1))
            (Default|GenerateNewOrder _asbp_delivery_game_instance)
            (Utilities|IsValid (Variables|Default|GetDeliveryWidget)
              (:Is%20Valid
                (Widget|RemovefromParent (Variables|Default|GetDeliveryWidget))))))
        (else
          (Development|PrintString "ここじゃない"))))))

(fn ConstructionScript)