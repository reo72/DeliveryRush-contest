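; BP_Register is an interactable register actor that empties the player's inventory when used.
; Any actor overlap enables input for player 0, sets PlayerNearby and shows a WB_RegisterPrompt widget; ending overlap reverses this.
; Pressing F while nearby clears PlayerInventory on BP_DeliveryGameInstance and removes the prompt.
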(event EventBeginPlay)

(event Collision|EventActorBeginOverlap
  (params (OtherActor :type Actor%20Object%20Reference))
  (Input|EnableInput (Game|GetPlayerController 0))
  (Variables|Default|SetbPlayerNearby true)
  (bind _returnvalue (UserInterface|CreateWidget "/Game/MJ/system/WB_RegisterPrompt.WB_RegisterPrompt_C"))
  (bind _output_get (Variables|Default|SetRegisterWidget _returnvalue))
  (UserInterface|Viewport|AddtoViewport _output_get 0))

(event EventTick
  (params (DeltaSeconds :type Float%20%28single-precision%29)))

(event Collision|EventActorEndOverlap
  (params (OtherActor :type Actor%20Object%20Reference))
  (Input|DisableInput (Game|GetPlayerController 0))
  (Variables|Default|SetbPlayerNearby false)
  (Utilities|IsValid 0
    (:Is%20Valid
      (Widget|RemovefromParent (Variables|Default|GetRegisterWidget)))))

(event Input|KeyboardEvents|F
  (params (Key :type Key%20Structure :default "None"))
  (:Pressed
    (if (Variables|Default|GetbPlayerNearby)
      (bind _asbp_delivery_game_instance (Utilities|Casting|CastToBP_DeliveryGameInstance (Game|GetGameInstance)))
      (Utilities|Array|Clear (Variables|/Game/MJ/system/BP_DeliveryGameInstance.BP_DeliveryGameInstance_C|GetPlayerInventory _asbp_delivery_game_instance))
      (Utilities|IsValid (Variables|Default|GetRegisterWidget)
        (:Is%20Valid
          (Widget|RemovefromParent (Variables|Default|GetRegisterWidget)))))))

(fn ConstructionScript)